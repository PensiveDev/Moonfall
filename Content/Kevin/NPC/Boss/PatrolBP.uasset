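; Griffon boss NPC character that takes damage, dies and plays a claw melee attack montage through a MeleeAttack event.
; AnyDamage plays a hit montage, subtracts Health, prints it and spawns a screen-projected CombatText damage widget, unless a fly-hit montage is playing.
; Health is checked before subtraction, so death triggers on the hit after it reaches zero.
; Death stops movement, plays the death montage and destroys the actor just before it ends.
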(event EventBeginPlay)

(event Collision|EventActorBeginOverlap
  (params (OtherActor :type Actor%20Object%20Reference)))

(event EventTick
  (params (DeltaSeconds :type Float%20%28single-precision%29)))

(event Game|Damage|EventAnyDamage
  (params (Damage :type Float%20%28single-precision%29) (DamageType :type Damage%20Type%20Object%20Reference) (InstigatedBy :type Controller%20Object%20Reference) (DamageCauser :type Actor%20Object%20Reference))
  (if (not (Variables|Default|GetisDying))
    (if (<= (Variables|Default|GetHealth) 0.0)
      ;[1 1 1] Death anim + depop
      (bind _returnvalue (Animation|PlayAnimMontage "/Game/QuadrapedCreatures/Griffon/Animations/ANIM_Griffon_Death_Montage.ANIM_Griffon_Death_Montage" 1.0 "None"))
      (Components|Movement|StopMovementImmediately (Variables|Character|GetCharacterMovement))
      (Variables|Default|SetisDying true)
      (Utilities|FlowControl|Delay (- _returnvalue 0.5))
      (Actor|DestroyActor)
      (elif (not (Animation|Montage|MontageIsPlaying (Components|SkeletalMesh|GetAnimInstance (Variables|Character|GetMesh)) "/Game/QuadrapedCreatures/Griffon/Animations/ANIM_Griffon_FlyGetHitStationary_Montage.ANIM_Griffon_FlyGetHitStationary_Montage"))
        (bind _returnvalue_2 (Animation|PlayAnimMontage "/Game/QuadrapedCreatures/Griffon/Animations/ANIM_Griffon_GetHit1_Montage.ANIM_Griffon_GetHit1_Montage" 1.0 "None"))
        (bind _output_get (Variables|Default|SetHealth (- (Variables|Default|GetHealth) Damage)))
        (Development|PrintString (Utilities|String|ToString(Float) _output_get))
        (CallFunction|SpawnCombatText (Transformation|GetActorLocation) Damage)
        (Utilities|FlowControl|Delay (+ _returnvalue_2 1.0))
        (Variables|Default|SetIsTakingDamages false)))))

(event EventMeleeAttack
  (Animation|PlayAnimMontage "/Game/QuadrapedCreatures/Griffon/Animations/ANIM_Griffon_LeftClawsAttack_RM_Montage.ANIM_Griffon_LeftClawsAttack_RM_Montage" 1.0 "None"))

(fn ConstructionScript)

(fn SpawnCombatText
  (params (WorldLocation :type Vector) (Damages :type Float%20%28single-precision%29))
  ;[1 1 1] Spawn Numbers  for damages
  (bind _returnvalue (UserInterface|CreateWidget "/Game/Kevin/Damages/CombatText.CombatText_C" 0 (.ScreenPosition (Class|GameplayStatics|ProjectWorldtoScreen (Game|GetPlayerController 0) WorldLocation false)) Damages))
  (UserInterface|Viewport|AddtoViewport _returnvalue 0))